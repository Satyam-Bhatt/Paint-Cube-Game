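; BP_MyGameMode is a game mode Blueprint that handles background music, the gameplay overlay and the win screen.
; BeginPlay plays the Background sound in 2D, while a persistent CreateSound2D alternative sits disconnected.
; The WinCondition event shows the cursor, creates WBP_Win, switches to UI-only input and adds the widget to the viewport.
; AddOverlay puts WBP_Gameplay on screen but is not called within this Blueprint.
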(event EventBeginPlay
  (Audio|PlaySound2D "/Game/Music/Background.Background" 1.0 1.0 0.0 0 0))

(event EventTick
  (params (DeltaSeconds :type Float%20%28single-precision%29)))

(event EventWinCondition
  (Variables|/Script/Engine.PlayerController|SetbShowMouseCursor (Game|GetPlayerController 0) true)
  (bind _returnvalue (UserInterface|CreateWidget "/Game/UI/WBP_Win.WBP_Win_C"))
  (Input|SetInputModeUIOnly (Game|GetPlayerController 0) _returnvalue "LockInFullscreen" false)
  (UserInterface|Viewport|AddtoViewport _returnvalue 0))

(fn ConstructionScript)

(fn AddOverlay
  (bind _returnvalue (UserInterface|CreateWidget "/Game/UI/WBP_Gameplay.WBP_Gameplay_C"))
  (UserInterface|Viewport|AddtoViewport _returnvalue 0))